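; Building base Blueprint for defence that resolves how much incoming damage a building actually takes.
; GetFinalDmg returns zero when the building cannot be attacked, and otherwise compares the damage type with the building's defense type.
; A matching type has the defense value subtracted and is floored at zero, while other types pass through at full value.
; The event graph is empty and construction only calls the parent.
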(event EventBeginPlay)

(event Collision|EventActorBeginOverlap
  (params (OtherActor :type Actor%20Object%20Reference)))

(event EventTick
  (params (DeltaSeconds :type Float%20%28single-precision%29)))

(fn ConstructionScript
  (|CallParentFunction))

(fn GetFinalDmg
  (params (Dmg_Type :type Byte) (Dmg_Value :type Float%20%28single-precision%29))
  (Variables|Default|SetDmg_Type Dmg_Type)
  (Variables|Default|SetDmg_Value Dmg_Value)
  (if (Variables|Default|GetCanbe_Attack)
    (if (== (Variables|Default|GetDmg_Type) (Variables|Default|GetDefense_Type))
      (Math|Float|CompareFloat (- (Variables|Default|GetDmg_Value) (Variables|Default|GetDefense_Value)) 0.0
        (:>
          (return (- (Variables|Default|GetDmg_Value) (Variables|Default|GetDefense_Value))))
        (:==
          (return 0.0))
        (:<
          (return 0.0)))
      (else
        (return (Variables|Default|GetDmg_Value))))
    (else
      (return 0.0))))
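; BP_BuildingBase_Attack is an attack building that attaches to its castle at a random offset and elevated height, firing bullets toward the castle's look-at point.
; Each tick it yaws the attack part and rolls the static mesh to aim at that point.
; Shoot spawns a BP_Bullet_Base from the gun position, gated by a CanShot flag that ReLoad restores after a reload delay.
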(event Custom|Shoot
  (bind _gunpos (Variables|Default|GetGunPos))
  (bind _returnvalue (Transformation|GetWorldTransform _gunpos))
  (if (Variables|Default|GetCanShot)
    (Game|SpawnActorfromClass "/Game/Blueprints/BuildingBase/BP_Bullet_Base.BP_Bullet_Base_C" (Math|Transform|MakeTransform (.location _returnvalue) (Math|Rotator|FindLookatRotation (.location _returnvalue) (Variables|/Game/Blueprints/ControlSystem/BP_CastlePawn.BP_CastlePawn_C|GetLookingAtLocation (Variables|Default|GetPrensentCastle))) "1,1,1") "Undefined" 0 0)
    (Variables|Default|SetCanShot false)
    (Development|PrintString "Hello")
    (CallFunction|ReLoad)))

(event Custom|ReLoad
  (Utilities|FlowControl|Delay (Variables|Default|GetReloadTime))
  (Development|PrintString "FinishReloading")
  (Variables|Default|SetCanShot true))

(event EventBeginPlay
  (bind _self self)
  (Transformation|AttachActorToActor _self (Variables|Default|GetPrensentCastle) "None" "KeepRelative" "KeepRelative" "KeepRelative" true)
  (Transformation|SetActorRelativeLocation _self (Math|Vector|MakeVector (Math|Random|RandomFloatinRange -5e+02 5e+02) (Math|Random|RandomFloatinRange -5e+02 5e+02) 1.44e+03))
  (Variables|Default|SetCanShot true))

(event EventTick
  (params (DeltaSeconds :type Float%20%28single-precision%29))
  (bind _attackpart (Variables|Default|GetAttackPart))
  (bind _staticmesh (Variables|Default|GetStaticMesh))
  (Transformation|SetWorldRotation _attackpart (Math|Rotator|MakeRotator 0.0 0.0 (+ (.Yaw (Math|Rotator|BreakRotator (Math|Rotator|FindLookatRotation (Transformation|GetWorldLocation _attackpart) (Variables|/Game/Blueprints/ControlSystem/BP_CastlePawn.BP_CastlePawn_C|GetLookingAtLocation (Variables|Default|GetPrensentCastle))))) -9e+01)) false false)
  (Transformation|SetRelativeRotation _staticmesh (Math|Rotator|MakeRotator (+ (.Roll (Math|Rotator|BreakRotator (Math|Rotator|FindLookatRotation (Transformation|GetWorldLocation _staticmesh) (Variables|/Game/Blueprints/ControlSystem/BP_CastlePawn.BP_CastlePawn_C|GetLookingAtLocation (Variables|Default|GetPrensentCastle))))) 9e+01) 0.0 0.0) false false))

(fn ConstructionScript
  (|CallParentFunction))
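; Player-controlled castle pawn with an orbit and zoom spring arm camera and switchable movement schemes.
; With MoveMode on, input axes offset the actor along its Arrow directions.
; Otherwise, gear inputs set horizontal and vertical target speeds, which Tick approaches in fixed acceleration steps.
; MoveMode2Mode then selects swept forward-and-strafe movement or unswept tank-like driving, where vertical speed becomes yaw.
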(event EventTick
  (params (DeltaSeconds :type Float%20%28single-precision%29))
  (if (not (Variables|Default|GetMoveMode))
    (Utilities|FlowControl|Sequence
      (:then_0
        (|UpDateMaxSpeed))
      (:then_1
        (|Acceleration))
      (:then_2
        (if (Variables|Default|GetMoveMode2Mode)
          (|MoveFunction1)
          (else
            (Transformation|AddActorWorldOffset self (* (Math|Vector|GetForwardVector (Variables|Default|GetArrow)) (Variables|Default|GetCurrentSpeed_Hor)))
            (Class|Actor|AddActorWorldRotation self (Math|Rotator|MakeRotator 0.0 0.0 (* (Variables|Default|GetCurrentSpeed_Ver) -0.01)))))))))

(event Input|ActionEvents|InputActionBS_ZoomDown
  (params (Key :type Key%20Structure))
  (bind _springarm (Variables|Default|GetSpringArm))
  ;[1 1 1] CameraControl
  (:Pressed
    (Variables|/Script/Engine.SpringArmComponent|SetTargetArmLength _springarm (+ (Variables|/Script/Engine.SpringArmComponent|GetTargetArmLength _springarm) 1e+02))))

(event Input|ActionEvents|InputActionBS_ZoomUp
  (params (Key :type Key%20Structure))
  (bind _springarm (Variables|Default|GetSpringArm))
  ;[1 1 1] CameraControl
  (:Pressed
    (Variables|/Script/Engine.SpringArmComponent|SetTargetArmLength _springarm (+ (Variables|/Script/Engine.SpringArmComponent|GetTargetArmLength _springarm) -1e+02))))

(event Input|ActionEvents|InputActionCS_SpeedUp_Hor
  (params (Key :type Key%20Structure))
  (bind _maxgear_hor (Variables|Default|GetMaxGear_Hor))
  ;[1 1 1] SwitchGear
  (:Pressed
    (bind _result (Math|Integer|IncrementInt (Variables|Default|GetCurrentGear_Hor))
      (:%20%20
        (Variables|Default|SetCurrentGear_Hor (Math|Integer|Clamp(Integer) _result (* _maxgear_hor -1) _maxgear_hor))
        (Variables|Default|SetIsIncreasing_Hor true)))))

(event Input|ActionEvents|InputActionCS_SpeedUp_Ver
  (params (Key :type Key%20Structure))
  (bind _maxgear_ver (Variables|Default|GetMaxGear_Ver))
  ;[1 1 1] SwitchGear
  (:Pressed
    (bind _result (Math|Integer|IncrementInt (Variables|Default|GetCurrentGear_Ver))
      (:%20%20
        (Variables|Default|SetCurrentGear_Ver (Math|Integer|Clamp(Integer) _result (* _maxgear_ver -1) _maxgear_ver))
        (Variables|Default|SetIsIncreasing_Ver true)))))

(event Input|ActionEvents|InputActionCS_SpeedDown_Ver
  (params (Key :type Key%20Structure))
  (bind _maxgear_ver (Variables|Default|GetMaxGear_Ver))
  ;[1 1 1] SwitchGear
  (:Pressed
    (bind _result (Math|Integer|DecrementInt (Variables|Default|GetCurrentGear_Ver))
      (:%20%20
        (Variables|Default|SetCurrentGear_Ver (Math|Integer|Clamp(Integer) _result (* _maxgear_ver -1) _maxgear_ver))
        (Variables|Default|SetIsIncreasing_Ver false)))))

(event Input|ActionEvents|InputActionCS_SpeedDown_Hor
  (params (Key :type Key%20Structure))
  (bind _maxgear_hor (Variables|Default|GetMaxGear_Hor))
  ;[1 1 1] SwitchGear
  (:Pressed
    (bind _result (Math|Integer|DecrementInt (Variables|Default|GetCurrentGear_Hor))
      (:%20%20
        (Variables|Default|SetCurrentGear_Hor (Math|Integer|Clamp(Integer) _result (* _maxgear_hor -1) _maxgear_hor))
        (Variables|Default|SetIsIncreasing_Hor false)))))

(event Input|AxisEvents|InputAxisCS_CameraRotationPitch
  (params (AxisValue :type Float%20%28single-precision%29))
  ;[1 1 1] CameraControl
  (Transformation|AddLocalRotation (Variables|Default|GetSpringArm) (Math|Rotator|MakeRotator 0.0 AxisValue 0.0) false false))

(event Input|AxisEvents|InputAxisCS_CameraRotationYaw
  (params (AxisValue :type Float%20%28single-precision%29))
  ;[1 1 1] CameraControl
  (Transformation|AddWorldRotation (Variables|Default|GetSpringArm) (Math|Rotator|MakeRotator 0.0 0.0 AxisValue) false false))

(event Input|AxisEvents|InputAxisCS_MoveForward
  (params (AxisValue :type Float%20%28single-precision%29))
  ;[1 1 1] MoveMode1
  (if (Variables|Default|GetMoveMode)
    (Transformation|AddActorWorldOffset self (* (* (Math|Vector|GetForwardVector (Variables|Default|GetArrow)) AxisValue) (Variables|Default|GetCurrentSpeed_Ver)))))

(event Input|AxisEvents|InputAxisCS_MoveRight
  (params (AxisValue :type Float%20%28single-precision%29))
  ;[1 1 1] MoveMode1
  (if (Variables|Default|GetMoveMode)
    (Transformation|AddActorWorldOffset self (* (* (Math|Vector|GetRightVector (Variables|Default|GetArrow)) AxisValue) (Variables|Default|GetCurrentSpeed_Hor)))))

(fn ConstructionScript)

(fn Accelerate
  (params (MaxSpeed :type Float%20%28single-precision%29) (CurrentSpeed :type Float%20%28single-precision%29) (IsIncreasing :type Boolean))
  (if (not (Math|Float|NearlyEqual(Float) MaxSpeed CurrentSpeed 0.5))
    (if IsIncreasing
      (return (+ CurrentSpeed (Variables|Default|GetAcceration)))
      (else
        (return (- CurrentSpeed (Variables|Default|GetAcceration)))))))
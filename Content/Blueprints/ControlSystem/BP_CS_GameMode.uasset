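; BP_CS_GameMode is a game mode that rebuilds a castle's saved buildings on a given actor.
; Its Initial event reads SavingInfo from BP_CastleInstance and looks up each entry's class in T_BuildingTable.
; It spawns each building at its saved offset from that actor, attaches it, and registers type 1 attack buildings in the actor's AttackBuildingArray.
; Debug prints trace the process, and key 6 prints the saved class names.
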(event Custom|Initial
  (params (PresentActor :type BP%20Castle%20Pawn%20Object%20Reference))
  (bind _asbp_castle_instance (Utilities|Casting|CastToBP_CastleInstance (Game|GetGameInstance))
    (:then
      (Development|PrintString "!!!!!!!!!!!")
      (for _array_element (Variables|/Game/Blueprints/BuidingSystem/BP_CastleInstance.BP_CastleInstance_C|GetSavingInfo _asbp_castle_instance)
        (Development|PrintString "Hello")
        (bind _returnvalue (Utilities|GetDataTableRow "/Game/Blueprints/BuildingBase/T_BuildingTable.T_BuildingTable" (.ClassName (Utilities|Struct|BreakS_SavingInfo _array_element)))
          (:then
            (Development|PrintString "foundSucessfully"))
          (:RowNotFound
            (Development|PrintString "NotFound")))
        (Utilities|FlowControl|Sequence
          (:then_0
            (bind _returnvalue_2 (Game|SpawnActorfromClass (.BuildingClass (Utilities|Struct|BreakS_BuildingTableInfo _returnvalue)) (Math|Transform|MakeTransform (+ (.RelativeLocation (Utilities|Struct|BreakS_SavingInfo _array_element)) (Transformation|GetActorLocation PresentActor)) "0, 0, 0" "1,1,1") "Undefined" 0 0))
            (Transformation|AttachActorToActor _returnvalue_2 PresentActor "None" "KeepWorld" "KeepRelative" "KeepRelative" true))
          (:then_1
            (if (== (.Type (Utilities|Struct|BreakS_BuildingTableInfo _returnvalue)) 1)
              (bind _asbp_building_base_attack (Utilities|Casting|CastToBP_BuildingBase_Attack _returnvalue_2))
              (Variables|/Game/Blueprints/BuildingBase/BP_BuildingBase_Attack.BP_BuildingBase_Attack_C|SetPrensentCastle _asbp_building_base_attack PresentActor)
              (Utilities|Array|Add (Variables|/Game/Blueprints/ControlSystem/BP_CastlePawn.BP_CastlePawn_C|GetAttackBuildingArray PresentActor) _asbp_building_base_attack))))))
    (:CastFailed
      (Development|PrintString "@@@@@@@@"))))

(event Input|KeyboardEvents|6
  (params (Key :type Key%20Structure))
  (:Pressed
    (bind _asbp_castle_instance (Utilities|Casting|CastToBP_CastleInstance (Game|GetGameInstance)))
    (for _array_element (Variables|/Game/Blueprints/BuidingSystem/BP_CastleInstance.BP_CastleInstance_C|GetSavingInfo _asbp_castle_instance)
      (Development|PrintString (Utilities|String|ToString(Name) (.ClassName (Utilities|Struct|BreakS_SavingInfo _array_element)))))))

(fn ConstructionScript)
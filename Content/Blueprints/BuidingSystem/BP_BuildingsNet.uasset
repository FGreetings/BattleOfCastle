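; BP_BuildingsNet is a grid cell for the building system that shows whether a building can be placed on it.
; BeginPlay gives its Cube a translucent grey dynamic M_Net material.
; Every Tick recolors it from IsbuildingOnIt and HasBuilding: red if occupied, green if free, grey when not targeted.
; Both flags are only read here; the Cube overlap events are empty, leaving older BP_BuildingBase overlap coloring disconnected.
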(event OnComponentBeginOverlap(Cube)
  (params (OverlappedComponent :type Primitive%20Component%20Object%20Reference) (OtherActor :type Actor%20Object%20Reference) (OtherComp :type Primitive%20Component%20Object%20Reference) (OtherBodyIndex :type Integer) (bFromSweep :type Boolean) (SweepResult :type Hit%20Result%20Structure%20%28by%20ref%29)))

(event OnComponentEndOverlap(Cube)
  (params (OverlappedComponent :type Primitive%20Component%20Object%20Reference) (OtherActor :type Actor%20Object%20Reference) (OtherComp :type Primitive%20Component%20Object%20Reference) (OtherBodyIndex :type Integer)))

(event Custom|ShowCanBuid
  (bind _netmaterial (Variables|Default|GetNetMaterial))
  (if (Variables|Default|GetHasBuilding)
    (Rendering|Material|SetVectorParameterValue _netmaterial "BaseColor" "(R=1.000000,G=0.000000,B=0.000000,A=1.000000)" :!class /Script/Engine.MaterialInstanceDynamic)
    (else
      (Rendering|Material|SetVectorParameterValue _netmaterial "BaseColor" "(R=0.000000,G=1.000000,B=0.000000,A=1.000000)" :!class /Script/Engine.MaterialInstanceDynamic))))

(event Custom|ShowCanBuildOff
  (Rendering|Material|SetVectorParameterValue (Variables|Default|GetNetMaterial) "BaseColor" "(R=0.484375,G=0.484375,B=0.484375,A=1.000000)" :!class /Script/Engine.MaterialInstanceDynamic))

(event Custom|ShowCannotBuild
  (Rendering|Material|SetVectorParameterValue (Variables|Default|GetNetMaterial) "BaseColor" "(R=1.000000,G=0.000000,B=0.000000,A=1.000000)" :!class /Script/Engine.MaterialInstanceDynamic))

(event EventBeginPlay
  (bind _returnvalue (Rendering|Material|CreateDynamicMaterialInstance (Variables|Default|GetCube) 0 "/Game/Blueprints/BuidingSystem/M_Net.M_Net" "None" :!class /Script/Engine.PrimitiveComponent))
  (bind _output_get (Variables|Default|SetNetMaterial _returnvalue))
  (Rendering|Material|SetVectorParameterValue _output_get "BaseColor" "(R=0.484375,G=0.484375,B=0.484375,A=1.000000)" :!class /Script/Engine.MaterialInstanceDynamic)
  (Rendering|Material|SetScalarParameterValue _output_get "Opacity" 0.3 :!class /Script/Engine.MaterialInstanceDynamic))

(event EventTick
  (params (DeltaSeconds :type Float%20%28single-precision%29))
  (if (Variables|Default|GetIsbuildingOnIt)
    (if (Variables|Default|GetHasBuilding)
      (CallFunction|ShowCannotBuild)
      (else
        (CallFunction|ShowCanBuid)))
    (else
      (CallFunction|ShowCanBuildOff))))

(fn ConstructionScript)
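; BP_BuildingCamera is the camera for the building system, providing rotation and zoom.
; Yaw and pitch axis inputs feed scaled controller rotation, which the actor follows through its use of control rotation.
; Zoom actions step the spring arm length within clamped limits.
; The construction script sets the arm's initial length, pitch and yaw from variables.
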(event Input|ActionEvents|InputActionBS_ZoomUp
  (params (Key :type Key%20Structure))
  (bind _springarm (Variables|Default|GetSpringArm))
  ;[1 1 1] RotateCamera(此Actor使用了control rotation）
  (:Pressed
    (Variables|/Script/Engine.SpringArmComponent|SetTargetArmLength _springarm (Math|Float|Clamp(Float) (+ (Variables|/Script/Engine.SpringArmComponent|GetTargetArmLength _springarm) -1e+02) 1e+03 1e+04))))

(event Input|ActionEvents|InputActionBS_ZoomDown
  (params (Key :type Key%20Structure))
  (bind _springarm (Variables|Default|GetSpringArm))
  ;[1 1 1] RotateCamera(此Actor使用了control rotation）
  (:Pressed
    (Variables|/Script/Engine.SpringArmComponent|SetTargetArmLength _springarm (Math|Float|Clamp(Float) (+ (Variables|/Script/Engine.SpringArmComponent|GetTargetArmLength _springarm) 1e+02) 1e+03 1e+04))))

(event Input|AxisEvents|InputAxisBS_CameraRotationPitch
  (params (AxisValue :type Float%20%28single-precision%29))
  ;[1 1 1] RotateCamera(此Actor使用了control rotation）
  (Pawn|Input|AddControllerPitchInput (* AxisValue 0.3)))

(event Input|AxisEvents|InputAxisBS_CameraRotationYaw
  (params (AxisValue :type Float%20%28single-precision%29))
  ;[1 1 1] RotateCamera(此Actor使用了control rotation）
  (Pawn|Input|AddControllerYawInput (* AxisValue 0.3)))

(fn ConstructionScript
  (bind _springarm (Variables|Default|GetSpringArm))
  (Variables|/Script/Engine.SpringArmComponent|SetTargetArmLength _springarm (Variables|Default|GetSpringArmLength))
  (Transformation|SetRelativeRotation _springarm (Math|Rotator|MakeRotator 0.0 (Variables|Default|GetSpringArmRoationPitch) (Variables|Default|GetSpringArmRotationYaw)) false false))
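; BP_Castle is a castle base for the building system that generates a grid of build cells around itself at BeginPlay.
; It spawns BP_BuildingsNet actors in nested loops sized by building area and NetSize, with small gaps and fixed offsets from its location.
; Each row is wrapped in an SNetWork struct to form a 2D NetWorkArray.
; It then registers itself as the present castle base on the BuildingSystemController.
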(event EventBeginPlay
  ;[1 1 1] Initial
  (Utilities|FlowControl|Sequence
    (:then_0
      (|生成建造网格))
    (:then_1
      (bind _asbuilding_system_controller (Utilities|Casting|CastToBuildingSystemController (Game|GetPlayerController 0)))
      (Variables|/Game/Blueprints/BuidingSystem/BuildingSystemController.BuildingSystemController_C|SetPresantCastelBase _asbuilding_system_controller self))))

(fn ConstructionScript)